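; BP_Enemigo4 is an enemy variant that inherits from the base enemy Blueprint and weaves sinusoidally as it descends.
; It overrides only Move, advancing X and Z along MovementVector scaled by Speed and DeltaTime.
; The Y step replaces that vector's component with a scaled degree-cosine of the current X position.
; This sideways step ignores DeltaTime, so the weave depends on how often Move runs.
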(event EventBeginPlay
  ;[1 1 1] Heredamos todo del BP_Enemy Base... pero sobreescribimos la función Move para crear otro movimiento en nuestro maquiavélico Enemigo_4.
  (|CallParentFunction) ; This node is disabled and will not be called.\nDrag off pins to build functionality.
)

(event Collision|EventActorBeginOverlap
  (params (OtherActor :type Actor%20Object%20Reference))
  ;[1 1 1] Heredamos todo del BP_Enemy Base... pero sobreescribimos la función Move para crear otro movimiento en nuestro maquiavélico Enemigo_4.
  (|CallParentFunction OtherActor) ; This node is disabled and will not be called.\nDrag off pins to build functionality.
)

(event EventTick
  (params (DeltaSeconds :type Float%20%28single-precision%29))
  ;[1 1 1] Heredamos todo del BP_Enemy Base... pero sobreescribimos la función Move para crear otro movimiento en nuestro maquiavélico Enemigo_4.
  (|CallParentFunction DeltaSeconds) ; This node is disabled and will not be called.\nDrag off pins to build functionality.
)

(fn ConstructionScript
  (|CallParentFunction))

(fn Move
  (params (Delta%20Time :type Float%20%28double-precision%29))
  (bind _returnvalue (Transformation|GetActorLocation))
  (bind _speed (Variables|Default|GetSpeed))
  (bind _movementvector (Variables|Default|GetMovementVector))
  (bind _returnvalue_2 (* Delta%20Time _speed))
  (bind _returnvalue_3 (* _returnvalue_2 _movementvector))
  ;[1 1 1] Le damos un movimiento sinusoidal al descenso de nuestro enemigo echando mano de la función Coseno aplicada a la componente x de su posición.
  (Transformation|SetActorLocation (+ (Math|Vector|MakeVector (.x _returnvalue) (.y _returnvalue) (.z _returnvalue)) (Math|Vector|MakeVector (.x _returnvalue_3) (* (Math|Trig|Cos(Degrees) (.x _returnvalue)) 2e+01) (.z _returnvalue_3))) false false))