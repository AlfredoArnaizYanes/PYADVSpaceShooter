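; Player projectile that flies forward along its facing direction at Speed, moved every Tick without sweep.
; On overlap, it destroys itself immediately against actors tagged Lateral and ignores Bonus-tagged actors and Pawns.
; Any other actor triggers an explosion emitter and sound, then the shot destroys itself after a short delay.
; The other actor is left untouched here, and each destruction prints a debug string.
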(event EventBeginPlay)

(event Collision|EventActorBeginOverlap
  (params (OtherActor :type Actor%20Object%20Reference))
  ;[1 1 1] Evento de colisión. Al colisionar con un enemigo ponemos efectos de sonido y explosión, y lo destruimos. El disparo del Player ignora a la Bonus y se destruye contra las paredes laterales
  (if (Utilities|Array|ContainsItem (Variables|/Script/Engine.Actor|GetTags OtherActor) "Lateral")
    (Actor|DestroyActor :!label _label)
    (Development|PrintString "Dispraro player destruido")
    (elif (not (Utilities|Array|ContainsItem (Variables|/Script/Engine.Actor|GetTags OtherActor) "Bonus"))
      (Utilities|Casting|CastToPawn OtherActor
        (:CastFailed
          (Effects|SpawnEmitteratLocation "/Game/StarterContent/Particles/P_Explosion.P_Explosion" (Transformation|GetActorLocation))
          (Audio|PlaySound2D "/Game/StarterContent/Audio/Explosion02.Explosion02" 1.0 1.0 0.0 0 0)
          (Utilities|FlowControl|Delay 0.2)
          (goto _label))))))

(event EventTick
  (params (DeltaSeconds :type Float%20%28single-precision%29))
  ;[1 1 1] El disparo del player se mueve en su eje x a velocidad Speed
  (Transformation|SetActorLocation (+ (Transformation|GetActorLocation) (* (Transformation|GetActorForwardVector) (* DeltaSeconds (Variables|Default|GetSpeed)))) false false))

(fn ConstructionScript)