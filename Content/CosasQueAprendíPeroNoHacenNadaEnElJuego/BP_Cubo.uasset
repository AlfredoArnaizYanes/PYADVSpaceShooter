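; BP_Cubo is a learning test kept for reference, unused in the game, showing keyboard movement for actors without Character Movement.
; BeginPlay adds an Enhanced Input mapping context to its player controller.
; Movement input is saved as a 2D value and cleared on release or cancel.
; Tick offsets the location along right and forward vectors by speed and delta time, without sweep; fire input only prints a message.
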(event Input|EnhancedActionEvents|EnhancedInputActionBP_InputFire
  (params (ActionValue :type Boolean) (ElapsedSeconds :type Float%20%28double-precision%29) (TriggeredSeconds :type Float%20%28double-precision%29) (InputAction :type Input%20Action%20Object%20Reference :default "/Game/BP_InputFire.BP_InputFire"))
  ;[1 1 1] Logica de movimiento por teclado para actores que no tienen Character Movement con Enhanced Input. En este proyecto no sirve para nada, pero me lo guardo
  (:Started
    (Development|PrintString "Disparo")))

(event Input|EnhancedActionEvents|EnhancedInputActionBP_InputMovement
  (params (ActionValue :type Vector%202D%20Structure) (ElapsedSeconds :type Float%20%28double-precision%29) (TriggeredSeconds :type Float%20%28double-precision%29) (InputAction :type Input%20Action%20Object%20Reference :default "/Game/BP_InputMovement.BP_InputMovement"))
  ;[1 1 1] Logica de movimiento por teclado para actores que no tienen Character Movement con Enhanced Input. En este proyecto no sirve para nada, pero me lo guardo
  (:Triggered
    (Variables|Default|SetInputSaved ActionValue))
  (:Canceled
    (Variables|Default|SetInputSaved "" :!label _label))
  (:Completed
    (goto _label)))

(event EventBeginPlay
  ;[1 1 1] Logica de movimiento por teclado para actores que no tienen Character Movement con Enhanced Input. En este proyecto no sirve para nada, pero me lo guardo
  (bind _asplayer_controller (Utilities|Casting|CastToPlayerController (Pawn|GetController)))
  (Utilities|IsValid (PlayerController|LocalPlayerSubsystems|GetEnhancedInputLocalPlayerSubsystem _asplayer_controller)
    (:Is%20Valid
      (Input|AddMappingContext (PlayerController|LocalPlayerSubsystems|GetEnhancedInputLocalPlayerSubsystem _asplayer_controller) "/Game/BP_InputMapping.BP_InputMapping" 0 "(bIgnoreAllPressedKeysUntilRelease=True,bForceImmediately=False,bNotifyUserSettings=False)"))))

(event EventTick
  (params (DeltaSeconds :type Float%20%28single-precision%29))
  (bind _speed (Variables|Default|GetSpeed))
  (bind _inputsaved (Variables|Default|GetInputSaved))
  (bind _returnvalue (* DeltaSeconds _speed))
  ;[1 1 1] Logica de movimiento por teclado para actores que no tienen Character Movement con Enhanced Input. En este proyecto no sirve para nada, pero me lo guardo
  (Transformation|SetActorLocation (+ (+ (* (Transformation|GetActorRightVector) (* _returnvalue (.x _inputsaved))) (* (* _returnvalue (.y _inputsaved)) (Transformation|GetActorForwardVector))) (Transformation|GetActorLocation)) false false))

(fn ConstructionScript)