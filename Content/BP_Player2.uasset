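; BP_Player2 is the player actor, which moves, fires projectiles and tracks lives.
; Enhanced Input, mapped on BeginPlay, drives movement along the actor's axes and firing from FirePoint, with a timer-gated cooldown.
; Overlaps with tagged actors destroy them: enemies cost a life, while BonusVida pickups add one up to a cap.
; At zero lives it calls Morimos on BP_GameModeLevel1.
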(event Custom|UpdateFire
  ;[1 1 1] Disparamos
  (Variables|Default|SetCanFire true))

(event Custom|SufrimosDaño
  (bind _output_get (Variables|Default|SetLifes (- (Variables|Default|GetLifes) 1)))
  (if (== _output_get 0)
    (bind _asbp_game_mode_level_1 (Utilities|Casting|CastToBP_GameModeLevel1 (Game|GetGameMode)))
    (Default|Morimos _asbp_game_mode_level_1)))

(event Input|EnhancedActionEvents|EnhancedInputActionBP_InputMovement
  (params (ActionValue :type Vector%202D%20Structure) (ElapsedSeconds :type Float%20%28double-precision%29) (TriggeredSeconds :type Float%20%28double-precision%29) (InputAction :type Input%20Action%20Object%20Reference :default "/Game/BP_InputMovement.BP_InputMovement"))
  ;[1 1 1] Movemos al player
  (Pawn|Input|AddMovementInput (Transformation|GetActorRightVector) (.x ActionValue) false)
  (Pawn|Input|AddMovementInput (Transformation|GetActorForwardVector) (.y ActionValue) false))

(event Input|EnhancedActionEvents|EnhancedInputActionBP_InputFire
  (params (ActionValue :type Boolean) (ElapsedSeconds :type Float%20%28double-precision%29) (TriggeredSeconds :type Float%20%28double-precision%29) (InputAction :type Input%20Action%20Object%20Reference :default "/Game/BP_InputFire.BP_InputFire"))
  ;[1 1 1] Disparamos
  (if (Variables|Default|GetCanFire)
    (CallFunction|DoFire)
    (Variables|Default|SetCanFire false)
    (Utilities|Time|SetTimerbyEvent (delegate Custom|UpdateFire) (Variables|Default|GetFireDelay))))

(event EventBeginPlay
  (bind _asplayer_controller (Utilities|Casting|CastToPlayerController (Pawn|GetController)))
  (Utilities|IsValid (PlayerController|LocalPlayerSubsystems|GetEnhancedInputLocalPlayerSubsystem _asplayer_controller)
    (:Is%20Valid
      (Input|AddMappingContext (PlayerController|LocalPlayerSubsystems|GetEnhancedInputLocalPlayerSubsystem _asplayer_controller) "/Game/BP_InputMapping.BP_InputMapping" 0 "(bIgnoreAllPressedKeysUntilRelease=True,bForceImmediately=False,bNotifyUserSettings=False)")
      (Utilities|Casting|CastToBP_GameModeLevel1 (Game|GetGameMode)))))

(event Collision|EventActorBeginOverlap
  (params (OtherActor :type Actor%20Object%20Reference))
  (if (Utilities|Array|ContainsItem (Variables|/Script/Engine.Actor|GetTags OtherActor) "Enemy")
    (Actor|DestroyActor OtherActor)
    (CallFunction|SufrimosDaño)
    (elif (Utilities|Array|ContainsItem (Variables|/Script/Engine.Actor|GetTags OtherActor) "BonusVida")
      (Utilities|Casting|CastToBP_GameModeLevel1 (Game|GetGameMode))
      (Actor|DestroyActor OtherActor)
      (if (< (Variables|Default|GetLifes) 5)
        (Variables|Default|SetLifes (+ (Variables|Default|GetLifes) 1))))))

(event EventTick
  (params (DeltaSeconds :type Float%20%28single-precision%29)))

(fn ConstructionScript)

(fn DoFire
  (Game|SpawnActorfromClass (Variables|Default|GetAmmo) (Transformation|GetWorldTransform (Variables|Default|GetFirePoint)) "Undefined" "MultiplyWithRoot" 0 0))