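; BP_Enemigo3 is a child enemy Blueprint that descends diagonally and bounces off the side walls.
; BeginPlay sets the inherited MovementVector from forward plus a scaled, negated right vector, giving a shallow descent that starts left to right on screen.
; Overlapping an actor tagged "Lateral" flips the vector's Y and shortens DelayShoot on each bounce.
; Tick is disabled, and no movement or shooting logic appears in this graph.
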(event EventBeginPlay
  ;[1 1 1] Para el enemigo 3 obtamos por un movimiento en diagonal asignando al Movement Vector la suma de su Right Vector y su Forward Vector. Al Right Vector lo multiplicamos por -2 para que no descienda en 45º sino en unos 25º. Al multiplicar por -2 también comenzará moviendose de izquierda a derecha en la pantalla.
  (|CallParentFunction)
  (Variables|Default|SetMovementVector (+ (* (Transformation|GetActorRightVector) -2) (Transformation|GetActorForwardVector))))

(event EventTick
  (params (DeltaSeconds :type Float%20%28single-precision%29))
  (|CallParentFunction DeltaSeconds) ; This node is disabled and will not be called.\nDrag off pins to build functionality.
)

(event Collision|EventActorBeginOverlap
  (params (OtherActor :type Actor%20Object%20Reference))
  ;[1 1 1] Para este enemigo también hay que tener en cuenta las colisiones con los laterales. Basta con multiplicar la componente "y" por -1 para que reboten en la pared y sigan su descenso.
  (|CallParentFunction OtherActor)
  (if (Utilities|Array|ContainsItem (Variables|/Script/Engine.Actor|GetTags OtherActor) "Lateral")
    (Variables|Default|SetMovementVector (Math|Vector|MakeVector (.x (Variables|Default|GetMovementVector)) (* (.y (Variables|Default|GetMovementVector)) -1.0) (.z (Variables|Default|GetMovementVector))))
    (Variables|Default|SetDelayShoot (- (Variables|Default|GetDelayShoot) 0.1))))

(fn ConstructionScript
  (|CallParentFunction))