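; BP_RandomGenerator is an enemy spawner that spawns a random enemy on a looping timer set by TiempoSpawn.
; SpawnEnemigos picks a random scene component tagged "SpawnPoint" as the location.
; The enemy class is rolled from BP_GameModeLevel1's Level, clamped by MaxNumEnemigos, and mapped to BP_EnemigoBase or BP_Enemigo2, with a third option unset.
; Each spawned BP_EnemigoBase binds its destroy event to EnemyDestroyed, which is currently empty.
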(event Custom|Spawn
  (bind _enemigospawmed (CallFunction|SpawnEnemigos))
  (bind _asbp_enemigo_base (Utilities|Casting|CastToBP_EnemigoBase _enemigospawmed))
  (EventDispatchers|BindEventtoOnEnemyDestroy _asbp_enemigo_base (delegate Custom|Enemy%20Destroyed)))

(event Custom|Enemy%20Destroyed)

(event EventBeginPlay
  (Utilities|Time|SetTimerbyEvent (delegate Custom|Spawn) (Variables|Default|GetTiempoSpawn) true)
  (bind _asbp_game_mode_level_1 (Utilities|Casting|CastToBP_GameModeLevel1 (Game|GetGameMode)))
  (Variables|Default|SetMy_GameMode _asbp_game_mode_level_1))

(event Collision|EventActorBeginOverlap
  (params (OtherActor :type Actor%20Object%20Reference)))

(event EventTick
  (params (DeltaSeconds :type Float%20%28single-precision%29)))

(fn ConstructionScript)

(fn SpawnEnemigos
  (bind _returnvalue (Actor|GetComponentsbyTag "/Script/Engine.SceneComponent" "SpawnPoint"))
  (bind _class (CallFunction|GetClasstoSpawn (Math|Random|RandomInteger (Variables|/Game/BP_GameModeLevel1.BP_GameModeLevel1_C|GetLevel (Variables|Default|GetMy_GameMode)))))
  (bind _returnvalue_2 (Game|SpawnActorfromClass _class (Transformation|GetWorldTransform (Utilities|Array|Get(acopy) _returnvalue (Math|Random|RandomInteger (Utilities|Array|Length _returnvalue)))) "Undefined" "MultiplyWithRoot" 0 0))
  (return _returnvalue_2))

(fn GetClasstoSpawn
  (params (Type :type Integer))
  (return (Utilities|Select :Index (Math|Integer|Clamp(Integer) Type 0 (- (Variables|Default|GetMaxNumEnemigos) 1)) :Option%200 "/Game/BP_EnemigoBase.BP_EnemigoBase_C" :Option%201 "/Game/BP_Enemigo2.BP_Enemigo2_C" :Option%202 0)))