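; Level 1 game mode for a space shooter that tracks score, destroyed enemies and the current level.
; EnemyDestroyed adds a fixed score increment, bumps the kill count and raises the level on every tenth kill.
; Empezamos and Morimos forward game start and player death to BP_SpaceShooterHUD.
; An unconnected branch that would give an enemy bonus every fifth kill never runs.
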(event Custom|Morimos
  (bind _asbp_space_shooter_hud (Utilities|Casting|CastToBP_SpaceShooterHUD (HUD|GetHUD (Game|GetPlayerController 0))))
  (Default|EstamosMuertos _asbp_space_shooter_hud))

(event Custom|Enemy%20Destroyed
  (CallFunction|IncrementaScore)
  (CallFunction|IncrementaEnemigosDestruidos)
  (CallFunction|IncremenaNivel (Variables|Default|GetEnemigosDestruidos)))

(event Custom|Empezamos
  (bind _asbp_space_shooter_hud (Utilities|Casting|CastToBP_SpaceShooterHUD (HUD|GetHUD (Game|GetPlayerController 0))))
  (Default|VamosAEmpezar _asbp_space_shooter_hud))

(event EventTick
  (params (DeltaSeconds :type Float%20%28single-precision%29)))

(fn ConstructionScript)

(fn IncremenaNivel
  (params (Enemig :type Integer))
  (if (== (Math|Integer|%(Integer) Enemig 10) 0)
    (Variables|Default|SetLevel (+ (Variables|Default|GetLevel) 1))))

(fn IncrementaScore
  (Variables|Default|SetScore (+ (Variables|Default|GetScore) (Variables|Default|GetIncrementPerEnemy))))

(fn IncrementaEnemigosDestruidos
  (Variables|Default|SetEnemigosDestruidos (+ (Variables|Default|GetEnemigosDestruidos) 1)))