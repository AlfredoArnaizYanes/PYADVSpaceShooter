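; Base enemy that flies along its initial forward vector every Tick and spawns Ammo at PuntoDisparo on a timer.
; Overlapping an actor tagged Player fires OnEnemyDestroy, whose bound handler calls GiveBonus, notifies BP_GameModeLevel1, then destroys it after a short delay.
; GiveBonus reads the kill count before it increments, spawning a pickup on every fifth count including zero, with shot or life type picked deterministically by modulo.
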(event Custom|Destroyed_Event
  ;[1 1 1] Nada más comenzar, el enemigo avanza hacia nosotros, y le decimos que esté atento al evento de destruirse. Cuando escucha este evento,  suelta el Bonus si le toca y luego se destruye. Me hubiera gustado gestionar la aparición del Bonus desde el Game Mode, me parecía lo apropiado, pues desde allí se lleva la cuenta de enemigos destruidos, pero al tener que instanciar el Bonus antes de destruirse no encontré la manera.
  (bind _asbp_game_mode_level_1 (Utilities|Casting|CastToBP_GameModeLevel1 (Game|GetGameMode)))
  (CallFunction|GiveBonus (Variables|/Game/BP_GameModeLevel1.BP_GameModeLevel1_C|GetEnemigosDestruidos _asbp_game_mode_level_1))
  (Default|EnemyDestroyed _asbp_game_mode_level_1)
  (Utilities|FlowControl|Delay 0.1)
  (Actor|DestroyActor))

(event EventBeginPlay
  ;[1 1 1] Nada más comenzar, el enemigo avanza hacia nosotros, y le decimos que esté atento al evento de destruirse. Cuando escucha este evento,  suelta el Bonus si le toca y luego se destruye. Me hubiera gustado gestionar la aparición del Bonus desde el Game Mode, me parecía lo apropiado, pues desde allí se lleva la cuenta de enemigos destruidos, pero al tener que instanciar el Bonus antes de destruirse no encontré la manera.
  (Variables|Default|SetMovementVector (Transformation|GetActorForwardVector))
  (EventDispatchers|BindEventtoOnEnemyDestroy (delegate Custom|Destroyed_Event)))

(event Collision|EventActorBeginOverlap
  (params (OtherActor :type Actor%20Object%20Reference))
  ;[1 1 1] Si el enemigo colisiona contra algo que tenga la etiqueta Player, llama al evento Enemy Destroy, que es el que se encarga de destruirlo y si le toca, soltar el Bonus.
  (if (Utilities|Array|ContainsItem (Variables|/Script/Engine.Actor|GetTags OtherActor) "Player")
    (Default|CallOnEnemyDestroy)))

(event EventTick
  (params (DeltaSeconds :type Float%20%28single-precision%29))
  ;[1 1 1] El enemigo nunca se está quieto, en cada Tick se mueve y nos dispara.
  (CallFunction|Move DeltaSeconds)
  (bind _output_get (Variables|Default|SetShotCurrentTime (+ DeltaSeconds (Variables|Default|GetShotCurrentTime))))
  (if (> _output_get (Variables|Default|GetDelayShoot))
    (Variables|Default|SetShotCurrentTime 0.0)
    (CallFunction|Fire)))

(fn ConstructionScript)

(fn Move
  (params (Delta%20Time :type Float%20%28double-precision%29))
  ;[1 1 1] Elenemigo se mueve según le marca su MovementVector
  (Transformation|SetActorLocation (+ (Transformation|GetActorLocation) (* (* Delta%20Time (Variables|Default|GetSpeed)) (Variables|Default|GetMovementVector))) false false))

(fn Fire
  ;[1 1 1] El enemigo dispara, está preparado para cambiarle la rotación a los disparos si lo quisiéramos
  (Game|SpawnActorfromClass (Variables|Default|GetAmmo) (Transformation|GetWorldTransform (Variables|Default|GetPuntoDisparo)) "Undefined" "MultiplyWithRoot" 0 0)
  (Transformation|SetActorRotation (Transformation|GetActorRotation)))

(fn GiveBonus
  (params (Contador :type Integer))
  ;[1 1 1] El enemigo nos da bonus por cada 5 que mueren. Los instancia en el mismo lugar que lo hacía con los disparos. El tipo de Bonus que nos da hemos hecho que dependa también del número de enemigos muertos, sin mternos en números Random usamos el Select, en el que dos opciones son el Bonus Disparo y solo una el Bonus Vida, para que la secuencia de Bonus a lo largo del juego sea D-V-D-D-V-D-D-V-D-D-V...
  (if (== (Math|Integer|%(Integer) Contador 5) 0)
    (Game|SpawnActorfromClass (Utilities|Select :Index (Math|Integer|%(Integer) Contador (Variables|Default|GetNumBonus)) :Option%200 "/Game/BP_BonusDisparo.BP_BonusDisparo_C" :Option%201 "/Game/BP_BonusVida.BP_BonusVida_C" :Option%202 "/Game/BP_BonusDisparo.BP_BonusDisparo_C") (Transformation|GetWorldTransform (Variables|Default|GetPuntoDisparo)) "Undefined" "MultiplyWithRoot" 0 0)
    (Transformation|SetActorRotation (Transformation|GetActorRotation))))